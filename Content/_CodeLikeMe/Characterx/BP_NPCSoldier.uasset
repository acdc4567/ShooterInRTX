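; BP_NPCSoldier is an NPC soldier character that aims and fires a gun, overriding aiming and targeting from its parent class.
; The Fire event raises the aim and, after a short delay, tells the BPGun child actor to shoot; stopping cancels both immediately.
; With a valid Opponent, it applies fixed pitch and yaw offsets to the parent's aim rotation and targets that actor's location.
; Otherwise, it uses its own rotation and targets a point ahead of the gun.
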(event EventBeginPlay
  (|CallParentFunction) ; This node is disabled and will not be called.\nDrag off pins to build functionality.
)

(event Collision|EventActorBeginOverlap
  (params (OtherActor :type Actor%20Object%20Reference))
  (|CallParentFunction OtherActor) ; This node is disabled and will not be called.\nDrag off pins to build functionality.
)

(event EventTick
  (params (DeltaSeconds :type Float%20%28single-precision%29))
  (|CallParentFunction DeltaSeconds) ; This node is disabled and will not be called.\nDrag off pins to build functionality.
)

(event EventFire
  (params (StartStop :type Boolean))
  (bind _bp_gun (Variables|Default|GetBP_Gun))
  (bind _childactor (Variables|/Script/Engine.ChildActorComponent|GetChildActor _bp_gun))
  (if StartStop
    (CallFunction|AimDown true)
    (Utilities|FlowControl|Delay 0.5)
    (Class|BPIGun|Fire(Message) _childactor true)
    (else
      (CallFunction|AimDown false)
      (Class|BPIGun|Fire(Message) _childactor false))))

(fn ConstructionScript
  (|CallParentFunction))

(fn GetAimingRotation
  (bind _myrotation (|CallParentFunction))
  (Utilities|IsValid (Variables|Default|GetOpponent)
    (:Is%20Valid
      (return (Math|Rotator|MakeRotator (.Roll (Math|Rotator|BreakRotator _myrotation)) (+ (.Pitch (Math|Rotator|BreakRotator _myrotation)) -15.0) (+ (.Yaw (Math|Rotator|BreakRotator _myrotation)) -11.0))))
    (:Is%20Not%20Valid
      (return (Transformation|GetActorRotation)))))

(fn GetTargetLocation
  (bind _opponent (Variables|Default|GetOpponent))
  (bind _bp_gun (Variables|Default|GetBP_Gun))
  (Utilities|IsValid _opponent
    (:Is%20Valid
      (return (Transformation|GetActorLocation _opponent) true _opponent self))
    (:Is%20Not%20Valid
      (return (+ (* (Math|Vector|GetForwardVector _bp_gun) 1e+03) (Transformation|GetWorldLocation _bp_gun)) true 0 self))))