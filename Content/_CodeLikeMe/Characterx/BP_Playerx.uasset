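; Player character Blueprint that adds third-person camera aiming and crouching to a parent character class.
; Aiming toggles the HUD reticle, animation flag, controller-yaw rotation and pitch limits, easing the follow camera between normal and ADS booms.
; Crouch input switches movement mode and lowers the camera.
; Overrides supply control rotation for aiming and a camera-origin trace target along control rotation, reporting a hit even when nothing blocks.
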(event EventBeginPlay
  (|CallParentFunction) ; This node is disabled and will not be called.\nDrag off pins to build functionality.
)

(event Collision|EventActorBeginOverlap
  (params (OtherActor :type Actor%20Object%20Reference))
  (|CallParentFunction OtherActor) ; This node is disabled and will not be called.\nDrag off pins to build functionality.
)

(event EventTick
  (params (DeltaSeconds :type Float%20%28single-precision%29))
  (|CallParentFunction DeltaSeconds) ; This node is disabled and will not be called.\nDrag off pins to build functionality.
)

(event EventAimDown
  (params (Enable/Disable :type Boolean))
  (bind _returnvalue (Game|GetPlayerCameraManager 0))
  (bind _returnvalue_2 (Game|GetPlayerController 0))
  (bind _abp_soldierref (Variables|Default|GetABP_SoldierRef))
  (bind _returnvalue_3 (HUD|GetHUD _returnvalue_2))
  (if Enable/Disable
    (Transformation|SetActorRotation (Math|Rotator|MakeRotator 0.0 0.0 (.yaw (Pawn|GetControlRotation :!class /Script/Engine.Pawn))))
    (Class|BPIUI|ToggleReticle(Message) _returnvalue_3 true)
    (Class|BPIAnimation|QuickAim(Message) _abp_soldierref true)
    (Transformation|AttachComponentToComponent (Variables|Default|GetFollowCamera) (Variables|Default|GetCameraBoom_ADS) "None" "KeepWorld" "KeepWorld" "KeepWorld" true)
    (Variables|Default|SetbUseControllerRotationYaw true)
    (Variables|/Script/Engine.PlayerCameraManager|SetViewPitchMax _returnvalue 5e+01)
    (Variables|/Script/Engine.PlayerCameraManager|SetViewPitchMin _returnvalue -5e+01)
    (else
      (Class|BPIUI|ToggleReticle(Message) _returnvalue_3 false)
      (Class|BPIAnimation|QuickAim(Message) _abp_soldierref false)
      (Transformation|AttachComponentToComponent (Variables|Default|GetFollowCamera) (Variables|Default|GetCameraBoom) "None" "KeepWorld" "KeepWorld" "KeepWorld" true)
      (Variables|Default|SetbUseControllerRotationYaw false)
      (Variables|/Script/Engine.PlayerCameraManager|SetViewPitchMax _returnvalue 6e+01)
      (Variables|/Script/Engine.PlayerCameraManager|SetViewPitchMin _returnvalue -6e+01)))
  (Components|MoveComponentTo (Variables|Default|GetFollowCamera) "0, 0, 0" "0, 0, 0" true true 0.35 false))

(event Input|ActionEvents|InputActionToggleCrouch
  (params (Key :type Key%20Structure :default "None"))
  (bind _followcamera (Variables|Default|GetFollowCamera))
  (:Pressed
    (CallFunction|ChangeMovementModex (Utilities|Select :Index (Variables|Default|GetCurrentMovementMode) :NewEnumerator0 "NewEnumerator3" :NewEnumerator1 "NewEnumerator3" :NewEnumerator2 "NewEnumerator3" :NewEnumerator3 "NewEnumerator1" :NewEnumerator4 "NewEnumerator3"))
    (if (Utilities|Enum|Equal(Enum) (Variables|Default|GetCurrentMovementMode) "NewEnumerator3")
      (Transformation|SetRelativeLocation _followcamera "0, 0,-40.000000" false false)
      (else
        (Transformation|SetRelativeLocation _followcamera "0, 0, 0" false false)))))

(fn ConstructionScript
  (|CallParentFunction))

(fn GetTargetLocation
  (bind _returnvalue (Game|GetPlayerController 0))
  (bind _followcamera (Variables|Default|GetFollowCamera))
  (bind _returnvalue_2 (Pawn|GetControlRotation _returnvalue :!class /Script/Engine.Controller))
  (bind _returnvalue_3 (Transformation|GetWorldLocation _followcamera))
  (bind _returnvalue_4 (Math|Vector|GetForwardVector _returnvalue_2))
  (bind _returnvalue_5 (* _returnvalue_4 1e+05))
  (bind _returnvalue_6 (+ _returnvalue_3 _returnvalue_5))
  (bind _outhit (Collision|LineTraceByChannel _returnvalue_3 _returnvalue_6 "TraceTypeQuery3" false 0 "None"))
  (if (.bblockinghit _outhit)
    (return (.location _outhit) true (.hitactor _outhit) self)
    (else
      (return _returnvalue_6 true 0 self))))

(fn GetAimingRotation
  (return (Pawn|GetControlRotation :!class /Script/Engine.Pawn)))

(fn GetDesiredVelocity
  (bind _desiredvelocity (|CallParentFunction))
  (return _desiredvelocity))