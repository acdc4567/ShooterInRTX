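; AI controller for soldier characters that runs the BT_Soldier behavior tree and reacts to perceived enemies.
; Perception updates ask the pawn for its team ID and the sensed actor whether it is an enemy, via message calls.
; For enemies, gaining or losing perception toggles the CanSeeEnemy blackboard key and sets or clears the pawn's opponent.
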(event OnTargetPerceptionUpdated(AIPerception)
  (params (Actor :type Actor%20Object%20Reference) (Stimulus :type AI%20Stimulus%20Structure))
  (bind _returnvalue (Pawn|GetControlledPawn))
  (bind _idx (Class|BPICharacter|GetTeamID(Message) (Variables|Default|GetControllerdPawn)))
  (bind _positive (Class|BPICharacter|IsEnemy(Message) Actor _idx))
  (if _positive
    (if (.bSuccessfullySensed (Utilities|Struct|BreakAIStimulus Stimulus))
      (AI|Components|Blackboard|SetValueasBool (AI|GetBlackboard 0) (Utilities|Name|MakeLiteralName "CanSeeEnemy") true)
      (Class|BPICharacter|SetOpponent(Message) _returnvalue Actor)
      (else
        (AI|Components|Blackboard|SetValueasBool (AI|GetBlackboard 0) (Utilities|Name|MakeLiteralName "CanSeeEnemy") false)
        (Class|BPICharacter|SetOpponent(Message) _returnvalue)))))

(event EventBeginPlay
  (Variables|Default|SetControllerdPawn (Pawn|GetControlledPawn))
  (AI|RunBehaviorTree "/Game/_CodeLikeMe/AI/BT_Soldier.BT_Soldier"))

(event EventTick
  (params (DeltaSeconds :type Float%20%28single-precision%29)))

(fn ConstructionScript)