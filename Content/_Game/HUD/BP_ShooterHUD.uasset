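; BP_ShooterHUD is a HUD Blueprint that draws a green crosshair at the center of the screen.
; On DrawHUD it halves the screen size to find the center, then offsets by the crosshair half-width and half-height variables.
; It draws the Cross_Q_9 texture there at a fixed size with a green tint, using canvas drawing with no widgets.
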(event EventDrawHUD
  (params (SizeX :type Integer) (SizeY :type Integer))
  (bind _output_get (Variables|Default|SetScreenCenter (Math|Vector2D|MakeVector2D (Math|Conversions|ToFloat(Integer) (/ SizeX 2)) (Math|Conversions|ToFloat(Integer) (/ SizeY 2)))))
  (Canvas|DrawTexture "/Game/_Game/Textures/Textures/Icons/Crosshairs/Cross_Q_9.Cross_Q_9" (- (.X (Math|Vector2D|BreakVector2D _output_get)) (Variables|Default|GetCrosshairHalfWidth)) (- (.Y (Math|Vector2D|BreakVector2D _output_get)) (Variables|Default|GetCrosshairHalfHeight)) 64.0 64.0 0.0 0.0 1.0 1.0 "(R=0.156846,G=1.000000,B=0.096208,A=1.000000)"))

(fn ConstructionScript)